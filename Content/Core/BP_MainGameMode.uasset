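; Main game mode that starts the main menu and Nightwoods music, spawns hunter and werewolf, and handles completion of all shrines.
; Custom events spawn and possess the hunter at a set position, and spawn the werewolf and initialize its AI controller.
; The hunter's goal tracker fires a delegate when all shrines are done, killing the werewolf and opening a new map after a short delay.
; It also provides a function to quit the game.
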(event `self.ReceiveBeginPlay`
  (bind _asbp_game_instance (cast `/Game/Core/BP_GameInstance` (`GameplayStatics.GetGameInstance`)))
  (`/Game/Core/BP_GameInstance.Init MainMenu` _asbp_game_instance)
  (`GameplayStatics.PlaySound2D` "/Game/Sounds/night-woods.night-woods" 0.7 1.0 0.0 null null false))

(event `Spawn Player Event`
  (bind _returnvalue (`|SpawnActorFromClass` "/Game/Player/BP_Hunter.BP_Hunter_C" (`KismetMathLibrary.MakeTransform` (`self.PlayerSpawnPos`)) "Undefined" "MultiplyWithRoot" null null))
  (bind _output_get (set `self.Player` _returnvalue))
  (`Controller.Possess` (`GameplayStatics.GetPlayerController` 0) _output_get)
  (add `PlayerGoalTracker.OnAllShrinesDoneDelegate` (`/Game/Player/BP_Hunter.PlayerGoalTracker` (`self.Player`)) (delegate `OnAllShrinesDoneDelegate_Event`)))

(event `OnAllShrinesDoneDelegate_Event`
  (message `/Game/AI/Interfaces/BPI_EnemyAI.Die` (`self.Enemy`))
  (`KismetSystemLibrary.Delay` 3.0)
  (`GameplayStatics.OpenLevelBySoftObjectPtr` "/Game/Remove/NewMap.NewMap"))

(event `Spawn Enemy Event`
  (bind _returnvalue (`|SpawnActorFromClass` "/Game/AI/BP_Werwolf.BP_Werwolf_C" (`KismetMathLibrary.MakeTransform` (`self.EnemySpawnPos`)) "Undefined" "MultiplyWithRoot" null null))
  (bind _output_get (set `self.Enemy` _returnvalue))
  (bind _asbp_aicontroller_base (cast `/Game/AI/BP_AIControllerBase` (`AIBlueprintHelperLibrary.GetAIController` _output_get)))
  (`/Game/AI/BP_AIControllerBase.Init Enemy AI` _asbp_aicontroller_base))

(fn `ExitGame`
  (`KismetSystemLibrary.QuitGame` null "Quit"))

(fn `UserConstructionScript`)