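; BP_Shrine is an interactable shrine that lights up with fire when used, and CanInteract allows use only while HasRitualDone is false.
; Interact calls the parent implementation, then ActivateAllVFX switches on four fire and four ember effects.
; It also creates a dynamic material instance on the mesh to raise its emissive parameter, and plays attenuated fire ignition and fire sounds at the shrine's location.
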(event `self.Interact`
  (params (Interactor :type "Actor Object Reference"))
  (bind _returnvalue (`self.K2_GetActorLocation`))
  (`parent.Interact` Interactor)
  (`self.ActivateAllVFX`)
  (bind _returnvalue_2 (`PrimitiveComponent.CreateDynamicMaterialInstance` (`self.StaticMesh`) 0 (`PrimitiveComponent.GetMaterial` (`self.StaticMesh`) 0) "None"))
  (`MaterialInstanceDynamic.SetScalarParameterValue` _returnvalue_2 "EmissionParam" 25.0)
  (`GameplayStatics.PlaySoundAtLocation` "/Game/Sounds/FireStart.FireStart" _returnvalue (struct) 1.5 1.0 0.0 "/Game/Sounds/SA_Monster.SA_Monster" null null null)
  (`GameplayStatics.PlaySoundAtLocation` "/Game/Sounds/fire-sound.fire-sound" _returnvalue (struct) 0.5 1.0 0.0 "/Game/Sounds/SA_Fire.SA_Fire" null null null))

(fn `ActivateAllVFX`
  (`ActorComponent.Activate` (`self.NS_Fire_01`) false)
  (`ActorComponent.Activate` (`self.NS_Fire_02`) false)
  (`ActorComponent.Activate` (`self.NS_Fire_03`) false)
  (`ActorComponent.Activate` (`self.NS_Fire_04`) false)
  (`ActorComponent.Activate` (`self.NS_Fire_Embers_01`) false)
  (`ActorComponent.Activate` (`self.NS_Fire_Embers_04`) false)
  (`ActorComponent.Activate` (`self.NS_Fire_Embers_03`) false)
  (`ActorComponent.Activate` (`self.NS_Fire_Embers_02`) false))

(fn `CanInteract`
  (returns (ReturnValue :type Boolean))
  (return (not (`self.bHasRitualDone`))))

(fn `UserConstructionScript`)