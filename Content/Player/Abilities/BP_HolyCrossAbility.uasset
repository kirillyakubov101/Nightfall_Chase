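; BP_HolyCrossAbility is a player ability that raises a holy cross to frighten what is in front of the owner.
; On activation it plays a choir sound, shows the owner's cross mesh and starts a montage on its skeletal mesh.
; A forward sphere trace immediately sends a Fear message to the first actor hit.
; Montage completion hides the cross and unlocks the owner's ability queue, with owner communication through message calls.
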(event `self.ReceiveBeginPlay`
  (bind _mesh (message `/Game/Player/BPI_AbilityOwner.GetMatchingStaticMesh` (`self.GetOwner`) (`self.CrossSofRef`)))
  (set `self.Mesh` _mesh))

(event `self.Try Activate Ability Event`
  (bind _returnvalue (`self.GetOwner`))
  (bind _returnvalue_2 (`Actor.K2_GetActorLocation` _returnvalue))
  (`GameplayStatics.PlaySoundAtLocation` "/Game/Sounds/short-choir.short-choir" (`Actor.K2_GetActorLocation` (`self.GetOwner`)) (struct) 1.0 1.0 0.0 null null null null)
  (`SceneComponent.SetVisibility` (`self.Mesh`) true true)
  (bind _mesh (message `/Game/Player/BPI_AbilityOwner.GetOwnerPrimarySkeletalMesh` (`self.GetOwner`)))
  (`|PlayMontage` _mesh "/Game/Player/Animations/PistolIdle_UE_Montage.PistolIdle_UE_Montage"
    (:`then`
      (bind (_outhit _returnvalue_3) (`KismetSystemLibrary.SphereTraceSingle` _returnvalue_2 (+ _returnvalue_2 (* (`Actor.GetActorForwardVector` _returnvalue) 120.0)) 250.0 "TraceTypeQuery5"))
      (if _returnvalue_3
        (message `/Game/AI/Interfaces/BPI_EnemyAI.Fear` (`.HitActor` (`GameplayStatics.BreakHitResult` _outhit)))))
    (:`OnCompleted`
      (message `/Game/Player/BPI_AbilityOwner.UnlockAbilityQueue` (`self.GetOwner`))
      (`SceneComponent.SetVisibility` (`self.Mesh`) false true))))