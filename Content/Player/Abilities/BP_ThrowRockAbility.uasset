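; Player ability that throws a rock by playing a throw montage and spawning a stone projectile.
; On activation it gets the owner's skeletal mesh and spawn point through interface messages, then plays the montage from its ThrowStart section.
; The "Throw" notify spawns BP_StoneProjectile at the spawn point, and the "Stop" notify stops the montage.
; Only the montage's Interrupted callback unlocks the owner's ability queue.
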(event `self.Try Activate Ability Event`
  (bind _returnvalue (`self.GetOwner`))
  (bind _mesh (message `/Game/Player/BPI_AbilityOwner.GetOwnerPrimarySkeletalMesh` _returnvalue))
  (bind _transform (message `/Game/Player/BPI_AbilityOwner.GetProjectileSpawnPoint` _returnvalue))
  (bind _notifyname (`|PlayMontage` _mesh "/Game/Player/Animations/ThrowObject_UE_Montage.ThrowObject_UE_Montage" 1.0 0.0 "ThrowStart")
    (:`OnInterrupted`
      (message `/Game/Player/BPI_AbilityOwner.UnlockAbilityQueue` (`self.GetOwner`)))
    (:`OnNotifyBegin`
      (if (== "Throw" _notifyname)
        (`|SpawnActorFromClass` "/Game/Player/Projectile/BP_StoneProjectile.BP_StoneProjectile_C" (`SceneComponent.K2_GetComponentToWorld` _transform) "Undefined" "MultiplyWithRoot" null null)
        (elif (== "Stop" _notifyname)
          (bind _character (message `/Game/Player/BPI_AbilityOwner.GetOwnerCharacter` (`self.GetOwner`)))
          (`Character.StopAnimMontage` _character "/Game/Player/Animations/ThrowObject_UE_Montage.ThrowObject_UE_Montage"))))))