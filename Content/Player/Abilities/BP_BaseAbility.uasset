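; BP_BaseAbility is a base player ability that provides cooldown-gated activation.
; TryActivateAbility checks and clears CanActivateAbility, broadcasts OnAbilityActive with the cooldown duration, starts a cooldown timer, then calls the empty TryActivateAbilityEvent hook.
; ResetAbilityCooldown restores availability, and CanUseAbility exposes the current state.
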(event `Try Activate Ability Event`)

(fn `CanUseAbility`
  (returns (bCanActivateAbility :type Boolean))
  (return (`self.bCanActivateAbility`)))

(fn `ResetAbilityCooldown`
  (set `self.bCanActivateAbility` true))

(fn `Try Activate Ability`
  (if (`self.bCanActivateAbility`)
    (set `self.bCanActivateAbility` false)
    (`self.OnAbilityActive` (`self.AbilityCooldown`))
    (`KismetSystemLibrary.K2_SetTimerDelegate` (`|CreateDelegate` :!event `ResetAbilityCooldown`) (`self.AbilityCooldown`))
    (`self.Try Activate Ability Event`)))