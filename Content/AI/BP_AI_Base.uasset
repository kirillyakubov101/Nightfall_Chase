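; BP_AI_Base is a base AI character that exposes patrol route, movement speed and attack hooks.
; On BeginPlay it casts and caches its BP_AIControllerBase controller.
; GetPatrolRoute returns the stored route, and SetMovementSpeed maps an idle, walking, jogging or sprinting state to the character's max walk speed and returns it.
; AttackEvent is an empty stub.
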(event `self.ReceiveBeginPlay`
  (bind _asbp_aicontroller_base (cast `/Game/AI/BP_AIControllerBase` (`AIBlueprintHelperLibrary.GetAIController` self)))
  (set `self.AIController` _asbp_aicontroller_base))

(event `Attack Event`)

(fn `GetPatrolRoute`
  (returns (PatrolRoute :type "/Game/AI/PatrolRoute/BP_PatrolRoute Object Reference"))
  (return (`self.PatrolRoute`)))

(fn `SetMovementSpeed`
  (params (MSpeed :type "/Game/AI/Enums/E_MovementSpeed Enum" :default "NewEnumerator1"))
  (returns (NewSpeed :type "Float (double-precision)"))
  (bind _output_get (set `CharacterMovementComponent.MaxWalkSpeed` (select `/Game/AI/Enums/E_MovementSpeed` MSpeed :`NewEnumerator0` 250.0 :`NewEnumerator2` 520.0 :`NewEnumerator3` 700.0 :!type "Float (single-precision)") (`self.CharacterMovement`)))
  (return _output_get))

(fn `UserConstructionScript`)