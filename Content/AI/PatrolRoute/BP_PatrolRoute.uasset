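; BP_PatrolRoute is a patrol route for AI that exposes world-space waypoints along a spline.
; IncrementPatrolRoute steps the current index by a direction value and flips it at the last and first spline points, giving a back-and-forth path.
; GetSplinePointAsWorldPosition returns the world location of the current point.
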(event `Increment Patrol Route`
  (bind _output_get (set `self.CurrentSplineIndex` (+ (`self.CurrentSplineIndex`) (`self.Direction`))))
  (if (== (- (`SplineComponent.GetNumberOfSplinePoints` (`self.Spline`)) 1) _output_get)
    (set `self.Direction` -1)
    (elif (== (`self.CurrentSplineIndex`) 0)
      (set `self.Direction` 1))))

(fn `GetSplinePointAsWorldPosition`
  (returns (ReturnValue :type "Vector Structure"))
  (return (`SplineComponent.GetLocationAtSplinePoint` (`self.Spline`) (`self.CurrentSplineIndex`) "World")))

(fn `UserConstructionScript`)