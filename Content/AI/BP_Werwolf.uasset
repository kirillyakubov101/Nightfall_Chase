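; Werewolf AI enemy that finds a patrol route, scans for points of interest and kills its target with a melee attack.
; VisualScan howls and grows a decal through a timeline, then runs a debug-drawn sphere trace and passes any hit point to the AI controller.
; The attack montage's Hit notify sends the target a death message, and completion switches AI state.
; A DoOnce reset on audio finish replays monster sounds during movement without overlap.
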(event `OnAudioFinished_Event`
  (bind _scanposition (`self.ScanPosition`))
  (goto _label :!via `Reset`))

(event `self.ReceiveTick`
  (params (DeltaSeconds :type "Float (single-precision)"))
  (bind _scanposition (`self.ScanPosition`))
  (if (> (`KismetMathLibrary.VSizeXY` (`self.GetVelocity`)) 100.0)
    (`/Engine/EditorBlueprintResources/StandardMacros.DoOnce` false :!label _label
      (:`Completed`
        (bind _returnvalue (`GameplayStatics.SpawnSoundAttached` "/Game/Sounds/MS_Monster.MS_Monster" _scanposition "None" (`SceneComponent.K2_GetComponentLocation` _scanposition) (struct) "KeepRelativeOffset" true 0.4 1.0 0.0 null null))
        (add `AudioComponent.OnAudioFinished` _returnvalue (delegate `OnAudioFinished_Event`))))))

(event `self.ReceiveBeginPlay`
  (`parent.ReceiveBeginPlay`)
  (bind _returnvalue (`|SpawnActorFromClass` "/Game/Abilities/SC_ScanDecal.SC_ScanDecal_C" (`SceneComponent.K2_GetComponentToWorld` (`self.ScanPosition`)) "Undefined" "MultiplyWithRoot" self null))
  (bind _output_get (set `self.ScanDecal` _returnvalue))
  (`self.SetActorHiddenInGame` _output_get true)
  (`self.K2_SetActorRotation` _output_get (struct :`Pitch` 90.0) false)
  (`self.K2_AttachToComponent` (`self.ScanDecal`) (`self.ScanPosition`) "None" "KeepWorld" "KeepWorld" "KeepWorld" true)
  (bind _returnvalue_2 (`GameplayStatics.GetActorOfClass` "/Game/AI/PatrolRoute/BP_PatrolRoute.BP_PatrolRoute_C"))
  (set `self.PatrolRoute` _returnvalue_2))

(event `VisualScan`
  (bind _scandecal (`self.ScanDecal`))
  (bind _scandecal_2 (`self.ScanDecal`))
  (bind _returnvalue (`SceneComponent.K2_GetComponentLocation` (`self.ScanPosition`)))
  (`GameplayStatics.PlaySoundAtLocation` "/Game/Sounds/WolfHowl.WolfHowl" (`self.K2_GetActorLocation` self) (struct) 3.0 1.0 0.0 null null self null)
  (`/Engine/EditorBlueprintResources/StandardMacros.IsValid` _scandecal_2
    (:`Is Valid`
      (`self.SetActorHiddenInGame` _scandecal_2 false)
      (bind (_direction _alpha) (`Timeline|Timeline` :!via `PlayFromStart`)
        (:`Update`
          (bind _returnvalue_2 (`KismetMathLibrary.Lerp` 0.0 12.0 _alpha))
          (`SceneComponent.SetWorldScale3D` (`DecalActor.Decal` (`self.ScanDecal`)) (`KismetMathLibrary.MakeVector` 1.0 _returnvalue_2 _returnvalue_2)))
        (:`Finished`
          (`self.SetActorHiddenInGame` _scandecal true)
          (`SceneComponent.SetWorldScale3D` (`DecalActor.Decal` _scandecal) (0.0 0.0 0.0))
          (bind (_outhit _returnvalue_3) (`KismetSystemLibrary.SphereTraceSingle` :`Start` _returnvalue :`End` (+ _returnvalue (0.1 0.0 0.0)) :`Radius` 1900.0 :`TraceChannel` "TraceTypeQuery3" :`DrawDebugType` "ForDuration" :`DrawTime` 10.0))
          (if _returnvalue_3
            (`/Game/AI/BP_AIControllerBase.SetPointOfInterest` (`self.AIController`) (`.ImpactPoint` (`GameplayStatics.BreakHitResult` _outhit)))))))))

(event `self.Attack Event`
  (`parent.Attack Event`)
  (bind _notifyname (`|PlayMontage` (`self.Mesh`) "/Game/AI/Animations/AM_WerwolfHit.AM_WerwolfHit")
    (:`OnCompleted`
      (`/Game/AI/BP_AIControllerBase.SwitchState` (`self.AIController`) "NewEnumerator3"))
    (:`OnNotifyBegin`
      (if (== _notifyname "Hit")
        (message `/Game/Player/BPI_EntityDeath.DeathEvent` (`/Game/AI/BP_AIControllerBase.GetTargetActor` (`self.AIController`)))))))

(fn `UserConstructionScript`
  (`parent.UserConstructionScript`))