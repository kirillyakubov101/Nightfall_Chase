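; Base enemy AI controller that runs BT_Base and drives a Passive, Attacking or Investigate state in its blackboard.
; Perception updates check each actor's sight and hearing stimuli and switch state through SwitchState.
; Sight turns a passive or investigating enemy to Attacking, and losing a seen target switches to Investigate.
; Sound only moves passive enemies to Investigate, and the attack target is always player character 0.
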(event `Init Enemy AI`
  (`self.RunBehaviorTree` "/Game/AI/BT_Base.BT_Base")
  (`BlackboardComponent.SetValueAsObject` (`AIBlueprintHelperLibrary.GetBlackboard` null) (`self.PlayerCharKeyName`) (`GameplayStatics.GetPlayerCharacter` 0))
  (`BlackboardComponent.SetValueAsEnum` (`AIBlueprintHelperLibrary.GetBlackboard` null) (`self.EnemyStateKeyName`) (enumliteral `/Game/AI/Enums/E_EnemyState` "NewEnumerator0")))

(event `self.AIPerception.OnPerceptionUpdated`
  (params (UpdatedActors :type "Array of Actor Object Reference (by ref)"))
  (for _array_element UpdatedActors
    (`|ExecutionSequence`
      (:`then_0`
        (bind _successfully_sensed (`self.CanSenseActor` _array_element "NewEnumerator1"))
        (if _successfully_sensed
          (`self.HandleSensedSight`)
          (set `self.PlayerInsight` true)
          (elif (`self.PlayerInsight`)
            (set `self.PlayerInsight` false)
            (`self.SwitchState` "NewEnumerator2"))))
      (:`then_1`
        (bind _successfully_sensed_2 (`self.CanSenseActor` _array_element "NewEnumerator2"))
        (if _successfully_sensed_2
          (`self.HandleSensedSound`))))))

(fn `CanSenseActor`
  (params (Actor :type "Actor Object Reference") (Sense :type "/Game/AI/Enums/E_AISense Enum" :default "NewEnumerator0"))
  (returns (`Successfully Sensed` :type Boolean) (Stimulus :type "AIStimulus Structure"))
  (bind _info (`AIPerceptionComponent.GetActorsPerception` (`self.AIPerception`) Actor))
  (for _array_element (`.LastSensedStimuli` (break `ActorPerceptionBlueprintInfo` _info))
    (bind _returnvalue (`AIPerceptionSystem.GetSenseClassForStimulus` _array_element))
    (if (== _returnvalue (select `/Game/AI/Enums/E_AISense` Sense :`NewEnumerator1` "/Script/AIModule.AISense_Sight" :`NewEnumerator2` "/Script/AIModule.AISense_Hearing" :!type "Object Class Reference"))
      (return (`.bSuccessfullySensed` (break `AIStimulus` _array_element)) _array_element))))

(fn `GetCurrentState`
  (returns (State :type "/Game/AI/Enums/E_EnemyState Enum"))
  (bind _returnvalue (`AIBlueprintHelperLibrary.GetBlackboard` null))
  (`/Engine/EditorBlueprintResources/StandardMacros.IsValid` _returnvalue
    (:`Is Valid`
      (return (cast `/Game/AI/Enums/E_EnemyState` (`BlackboardComponent.GetValueAsEnum` _returnvalue (`self.EnemyStateKeyName`)))))))

(fn `HandleSensedSight`
  (switch `/Game/AI/Enums/E_EnemyState` (`self.GetCurrentState`)
    (:`NewEnumerator0`
      _)
    (:`NewEnumerator2`
      _))
  (`self.SwitchState` "NewEnumerator1"))

(fn `HandleSensedSound`
  (switch `/Game/AI/Enums/E_EnemyState` (`self.GetCurrentState`)
    (:`NewEnumerator0`
      (`self.SwitchState` "NewEnumerator2"))))

(fn `SwitchState`
  (params (State :type "/Game/AI/Enums/E_EnemyState Enum" :default "NewEnumerator0"))
  (bind _returnvalue (`AIBlueprintHelperLibrary.GetBlackboard` null))
  (`/Engine/EditorBlueprintResources/StandardMacros.IsValid` (`AIBlueprintHelperLibrary.GetBlackboard` null)
    (:`Is Valid`
      (switch `/Game/AI/Enums/E_EnemyState` State
        (:`NewEnumerator0`
          (`BlackboardComponent.SetValueAsEnum` (`AIBlueprintHelperLibrary.GetBlackboard` null) (`self.EnemyStateKeyName`) State))
        (:`NewEnumerator1`
          (`BlackboardComponent.SetValueAsEnum` _returnvalue (`self.EnemyStateKeyName`) State)
          (`BlackboardComponent.SetValueAsObject` _returnvalue (`self.PlayerCharKeyName`) (`GameplayStatics.GetPlayerCharacter` 0)))
        (:`NewEnumerator2`
          (`BlackboardComponent.SetValueAsEnum` (`AIBlueprintHelperLibrary.GetBlackboard` null) (`self.EnemyStateKeyName`) State))))))

(fn `UserConstructionScript`)